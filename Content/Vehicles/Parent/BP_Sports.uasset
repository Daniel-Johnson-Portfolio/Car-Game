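; Sports car vehicle Blueprint that extends a parent vehicle class with car-specific drivetrain data, exhausts and brake lights.
; After the parent BeginPlay, it sets gear ratios, final drive, tire diameter and the sport exhaust references.
; Brake input feeds the vehicle movement component and toggles BreakLights.
; BreakLights creates a new dynamic chassis material on every call, assigns it to mesh slot 0 and sets the brake light glow.
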(event `self.ReceiveBeginPlay`
  (`parent.ReceiveBeginPlay`)
  (set `self.GearRatios` (`|MakeArray` 2.86 0.0 4.89 3.17 2.15 1.56 1.18 0.94 0.76 0.61))
  (set `self.FinalDriveRatio` 3.33)
  (set `self.TireDiameter` 21.0)
  (set `self.LeftExhaust` (`self.LeftExhaustSport`))
  (set `self.RightExhaust` (`self.RightExhaustSport`)))

(event `/Game/BPI_Controll.Input_Breaking`
  (params (ActionValue :type "Float (double-precision)"))
  (if (== ActionValue 0.0)
    (`self.BreakLights` false)
    (else
      (`self.BreakLights` true)))
  (`ChaosVehicleMovementComponent.SetBrakeInput` (`self.VehicleMovementComponent`) ActionValue))

(fn `BreakLights`
  (params (`On/Off` :type Boolean))
  (bind _returnvalue (`KismetMaterialLibrary.CreateDynamicMaterialInstance` "/Game/Vehicles/VH_Sports/Materials/MI_SportsCar_Chassis.MI_SportsCar_Chassis" "None"))
  (`PrimitiveComponent.SetMaterial` (`self.Mesh`) 0 _returnvalue)
  (if `On/Off`
    (`MaterialInstanceDynamic.SetScalarParameterValue` _returnvalue "BrakeLightPower" 200.0)
    (else
      (`MaterialInstanceDynamic.SetScalarParameterValue` _returnvalue "BrakeLightPower" 4.0))))

(fn `UserConstructionScript`
  (`parent.UserConstructionScript`))