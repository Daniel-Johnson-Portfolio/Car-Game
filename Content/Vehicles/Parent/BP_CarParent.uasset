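; Parent Blueprint for drivable cars that routes throttle, brake, steering, handbrake and manual gear inputs to the vehicle movement component.
; Tick estimates RPM from forward speed, gear ratio, final drive and tire diameter, then flags a stall when revs fall below idle while moving.
; A UI interface widget found after BeginPlay receives RPM, gear, speed and handbrake updates.
; Upshifts spawn exhaust pops; ignition input and car switching are empty stubs.
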(event `self.ReceiveBeginPlay`
  (`KismetSystemLibrary.Delay` 0.2)
  (bind _foundwidgets (`WidgetBlueprintLibrary.GetAllWidgetsWithInterface` "/Game/BPI_UI.BPI_UI_C"))
  (for _array_element _foundwidgets
    (set `self.UserInterface` _array_element :!label _label))
  (goto _label))

(event `/Game/BPI_Controll.Input_Ignition`
  ;[1 1 1] Maybe Scrap For Sake Of Playablitiy
)

(event `/Game/BPI_Controll.Input_Handbreak`
  (params (Toggle :type Boolean))
  (`ChaosVehicleMovementComponent.SetHandbrakeInput` (`self.VehicleMovementComponent`) Toggle)
  (message `/Game/BPI_UI.UI_HandBreak` (`self.UserInterface`) Toggle))

(event `/Game/BPI_Controll.Input_Breaking`
  (params (ActionValue :type "Float (double-precision)"))
  (`ChaosVehicleMovementComponent.SetBrakeInput` (`self.VehicleMovementComponent`) ActionValue))

(event `/Game/BPI_Controll.Input_Steering`
  (params (ActionValue :type "Float (double-precision)"))
  (`ChaosVehicleMovementComponent.SetSteeringInput` (`self.VehicleMovementComponent`) ActionValue))

(event `/Game/BPI_Controll.Input_Forward`
  (params (ActionInput :type "Float (double-precision)"))
  (`ChaosVehicleMovementComponent.SetThrottleInput` (`self.VehicleMovementComponent`) ActionInput))

(event `/Game/BPI_Controll.Input_GearDown`
  (bind _vehiclemovementcomponent (`self.VehicleMovementComponent`))
  (`ChaosVehicleMovementComponent.SetTargetGear` _vehiclemovementcomponent (- (`ChaosVehicleMovementComponent.GetCurrentGear` _vehiclemovementcomponent) 1) false))

(event `/Game/BPI_Controll.Input_GearUp`
  (bind _vehiclemovementcomponent (`self.VehicleMovementComponent`))
  (`ChaosVehicleMovementComponent.SetTargetGear` _vehiclemovementcomponent (+ (`ChaosVehicleMovementComponent.GetCurrentGear` _vehiclemovementcomponent) 1) false)
  (`NiagaraFunctionLibrary.SpawnSystemAtLocation` "/Game/Vehicles/VH_Sports/VFX/NS_Pop.NS_Pop" (`SceneComponent.K2_GetComponentLocation` (`self.LeftExhaust`)))
  (`NiagaraFunctionLibrary.SpawnSystemAtLocation` "/Game/Vehicles/VH_Sports/VFX/NS_Pop.NS_Pop" (`SceneComponent.K2_GetComponentLocation` (`self.RightExhaust`))))

(event `self.ReceiveTick`
  (params (DeltaSeconds :type "Float (single-precision)"))
  (bind _vehiclemovementcomponent (`self.VehicleMovementComponent`))
  (bind _returnvalue (`ChaosVehicleMovementComponent.GetCurrentGear` _vehiclemovementcomponent))
  (bind _returnvalue_2 (/ (* (`ChaosVehicleMovementComponent.GetForwardSpeedMPH` _vehiclemovementcomponent) (`|GetArrayItem` (`self.GearRatios`) (- _returnvalue 1)) (`self.FinalDriveRatio`) 336.13) (`self.TireDiameter`)))
  ;[1 1 1] CalculatesRPM
  (`self.UI_Update`)
  (if (not (<= _returnvalue 0))
    (if (== _returnvalue 1)
      (set `self.RPM` (+ _returnvalue_2 (`self.IdleSpeed`)))
      (else
        (set `self.RPM` _returnvalue_2)))
    (if (`self.Ignition`)
      _
      (else
        _))
    (`self.StallCheck`)))

(event `StallCheck`
  (if (and (< (`self.RPM`) (- (`self.IdleSpeed`) 200.0)) (`self.Ignition`) (> (`ChaosVehicleMovementComponent.GetForwardSpeedMPH` (`self.VehicleMovementComponent`)) 1.0))
    (set `self.Ignition` false)
    (`KismetSystemLibrary.PrintString` "Stalled")))

(event `UI_Update`
  (bind _userinterface (`self.UserInterface`))
  (bind _vehiclemovementcomponent (`self.VehicleMovementComponent`))
  (message `/Game/BPI_UI.UI_RPM` _userinterface (`KismetMathLibrary.FTrunc` (`self.RPM`)))
  (message `/Game/BPI_UI.UI_Gear` _userinterface (`ChaosVehicleMovementComponent.GetCurrentGear` _vehiclemovementcomponent))
  (message `/Game/BPI_UI.UI_Speed` _userinterface (`KismetMathLibrary.FTrunc` (`ChaosVehicleMovementComponent.GetForwardSpeedMPH` _vehiclemovementcomponent))))

(fn `Input_SwitchCar`
  (params (CurrentCar :type "WheeledVehiclePawn Object Reference") (Player :type "PlayerController Object Reference"))
  (returns (NewCar :type "WheeledVehiclePawn Object Reference"))
  (return null))

(fn `UserConstructionScript`)