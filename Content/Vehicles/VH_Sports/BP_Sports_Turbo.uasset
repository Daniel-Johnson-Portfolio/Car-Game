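; Sports vehicle Blueprint that adds a turbo flutter sound when the throttle is released or the gear increases.
; Tick runs a repeating two-second timer that arms the turbo build-up flag.
; At high RPM with the flag set, either event plays the flutter and clears the flag, scaling volume by the current timer value.
; The timer resets only on arming, so volume follows its position in the cycle.
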(event `self.ReceiveTick`
  (params (DeltaSeconds :type "Float (single-precision)"))
  (bind _output_get (set `self.TurboBuildUpTime` (+ (`self.TurboBuildUpTime`) DeltaSeconds)))
  (if (> _output_get 2.0)
    (set `self.TurboBuildUp` true)
    (set `self.TurboBuildUpTime` 0.0))
  (`parent.ReceiveTick` DeltaSeconds))

(event `self.ThrottleReleased`
  (bind _turboflutter (`self.TurboFlutter`))
  (if (> (`self.RPM`) 5000.0) :!label _label
    (if (`self.TurboBuildUp`)
      (set `AudioComponent.VolumeMultiplier` (`KismetMathLibrary.MapRangeClamped` (`self.TurboBuildUpTime`) 0.0 5.0 0.0 0.3) _turboflutter)
      (`AudioComponent.Play` _turboflutter 0.0)
      (set `self.TurboBuildUp` false))))

(event `self.GearHasIncreased`
  (goto _label))

(fn `UserConstructionScript`
  (`parent.UserConstructionScript`))