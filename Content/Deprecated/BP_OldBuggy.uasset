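; Deprecated player-drivable buggy Blueprint that turns Enhanced Input actions into Chaos-style vehicle movement.
; BeginPlay adds its input mapping context to player 0.
; Throttle, brake, steering and handbrake values feed the vehicle movement component, while gear up and down step the target gear on completion.
; Tick prints forward speed in MPH and current gear as debug output.
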(event `self.ReceiveBeginPlay`
  (bind _returnvalue (pcsubsystem `EnhancedInputLocalPlayerSubsystem` (`GameplayStatics.GetPlayerController` 0)))
  (`/Engine/EditorBlueprintResources/StandardMacros.IsValid` _returnvalue
    (:`Is Valid`
      (`EnhancedInputSubsystemInterface.AddMappingContext` _returnvalue "/Game/Inputs/InputMappingContext.InputMappingContext" 0 (struct))
      (`KismetSystemLibrary.PrintString` "Hello"))))

(event `EnhancedInput|/Game/Inputs/Handbreak`
  (params (ActionValue :type Boolean) (ElapsedSeconds :type "Float (double-precision)") (TriggeredSeconds :type "Float (double-precision)") (InputAction :type "InputAction Object Reference" :default "/Game/Inputs/Handbreak.Handbreak"))
  (:`Triggered`
    (`ChaosVehicleMovementComponent.SetHandbrakeInput` (`self.VehicleMovementComponent`) ActionValue :!label _label))
  (:`Completed`
    (goto _label)))

(event `EnhancedInput|/Game/Inputs/Break`
  (params (ActionValue :type "Float (double-precision)") (ElapsedSeconds :type "Float (double-precision)") (TriggeredSeconds :type "Float (double-precision)") (InputAction :type "InputAction Object Reference" :default "/Game/Inputs/Break.Break"))
  (:`Triggered`
    (set `self.Brake` ActionValue)
    (`ChaosVehicleMovementComponent.SetBrakeInput` (`self.VehicleMovementComponent`) (`self.Brake`) :!label _label_2))
  (:`Completed`
    (set `self.Brake` ActionValue)
    (goto _label_2)))

(event `EnhancedInput|/Game/Inputs/Throttle`
  (params (ActionValue :type "Float (double-precision)") (ElapsedSeconds :type "Float (double-precision)") (TriggeredSeconds :type "Float (double-precision)") (InputAction :type "InputAction Object Reference" :default "/Game/Inputs/Throttle.Throttle"))
  (:`Triggered`
    (set `self.Throttle` ActionValue)
    (`ChaosVehicleMovementComponent.SetThrottleInput` (`self.VehicleMovementComponent`) (`self.Throttle`) :!label _label_3))
  (:`Completed`
    (set `self.Throttle` 0.0)
    (goto _label_3)))

(event `EnhancedInput|/Game/Inputs/Steering`
  (params (ActionValue :type "Float (double-precision)") (ElapsedSeconds :type "Float (double-precision)") (TriggeredSeconds :type "Float (double-precision)") (InputAction :type "InputAction Object Reference" :default "/Game/Inputs/Steering.Steering"))
  (:`Triggered`
    (set `self.Steering` ActionValue)
    (`ChaosVehicleMovementComponent.SetSteeringInput` (`self.VehicleMovementComponent`) (`self.Steering`) :!label _label_4))
  (:`Completed`
    (set `self.Steering` 0.0)
    (goto _label_4)))

(event `self.ReceiveTick`
  (params (DeltaSeconds :type "Float (single-precision)"))
  (bind _vehiclemovementcomponent (`self.VehicleMovementComponent`))
  (`KismetSystemLibrary.PrintString` (`KismetStringLibrary.Conv_DoubleToString` (`ChaosVehicleMovementComponent.GetForwardSpeedMPH` _vehiclemovementcomponent)))
  (`KismetSystemLibrary.PrintString` (`KismetStringLibrary.Conv_IntToString` (`ChaosVehicleMovementComponent.GetCurrentGear` _vehiclemovementcomponent))))

(event `EnhancedInput|/Game/Inputs/GearUp`
  (params (ActionValue :type Boolean) (ElapsedSeconds :type "Float (double-precision)") (TriggeredSeconds :type "Float (double-precision)") (InputAction :type "InputAction Object Reference" :default "/Game/Inputs/GearUp.GearUp"))
  (bind _vehiclemovementcomponent (`self.VehicleMovementComponent`))
  (:`Completed`
    (`ChaosVehicleMovementComponent.SetTargetGear` _vehiclemovementcomponent (+ (`ChaosVehicleMovementComponent.GetCurrentGear` _vehiclemovementcomponent) 1) false)))

(event `EnhancedInput|/Game/Inputs/GearDown`
  (params (ActionValue :type Boolean) (ElapsedSeconds :type "Float (double-precision)") (TriggeredSeconds :type "Float (double-precision)") (InputAction :type "InputAction Object Reference" :default "/Game/Inputs/GearDown.GearDown"))
  (bind _vehiclemovementcomponent (`self.VehicleMovementComponent`))
  (:`Completed`
    (`ChaosVehicleMovementComponent.SetTargetGear` _vehiclemovementcomponent (- (`ChaosVehicleMovementComponent.GetCurrentGear` _vehiclemovementcomponent) 1) false)))

(fn `UserConstructionScript`)