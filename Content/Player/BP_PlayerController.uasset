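; Player controller for the driving game that spawns and possesses the player's car, creates the UI and spawns the goal.
; The GameInstance supplies the sports car mod variant and the part materials applied on setup.
; CarSwitcher replaces the current car in place using a class map, falling back to the stock sports car.
; Enhanced Input drives the switch menu and mouse camera swivel, forwarding driving controls to the pawn through interface messages.
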(event `SpawnCar`
  (bind _defaultspawn (`self.DefaultSpawn`))
  ;[1 1 1] Spawns Defualt Car At a spwan position
  (bind _carmod (message `/Game/Managers/BPI_GetManager.ReturnCarMods` (`GameplayStatics.GetGameInstance`)))
  (switch `/Game/Vehicles/CarMods` _carmod
    (:`NewEnumerator0`
      (bind _returnvalue (`|SpawnActorFromClass` "/Game/Vehicles/VH_Sports/BP_Sports.BP_Sports_C" _defaultspawn "AdjustIfPossibleButAlwaysSpawn" "MultiplyWithRoot" null null))
      (`self.SetUpCar` _returnvalue))
    (:`NewEnumerator1`
      (bind _returnvalue_2 (`|SpawnActorFromClass` "/Game/Vehicles/VH_Sports/BP_Sports_SuperCharged.BP_Sports_SuperCharged_C" _defaultspawn "AdjustIfPossibleButAlwaysSpawn" "MultiplyWithRoot" null null))
      (`self.SetUpCar` _returnvalue_2))
    (:`NewEnumerator2`
      (bind _returnvalue_3 (`|SpawnActorFromClass` "/Game/Vehicles/VH_Sports/BP_Sports_Turbo.BP_Sports_Turbo_C" _defaultspawn "AdjustIfPossibleButAlwaysSpawn" "MultiplyWithRoot" null null))
      (`self.SetUpCar` _returnvalue_3))
    (:`NewEnumerator3`
      (bind _returnvalue_4 (`|SpawnActorFromClass` "/Game/Vehicles/VH_Sports/BP_Sports_Rasied.BP_Sports_Rasied_C" _defaultspawn "AdjustIfPossibleButAlwaysSpawn" "MultiplyWithRoot" null null))
      (`self.SetUpCar` _returnvalue_4))))

(event `self.ReceiveBeginPlay`
  (bind _returnvalue (pcsubsystem `EnhancedInputLocalPlayerSubsystem` self))
  (`self.SpawnCar`)
  (`self.Initialise UI`)
  (bind _returnvalue_2 (`|SpawnActorFromClass` "/Game/Levels/TerrainLevel/BP_Goal.BP_Goal_C" (`self.GoalPosistion`) "Undefined" "MultiplyWithRoot" null null))
  (set `/Game/Levels/TerrainLevel/BP_Goal.GoalUI` (`self.UI`) _returnvalue_2)
  (`/Engine/EditorBlueprintResources/StandardMacros.IsValid` _returnvalue
    (:`Is Valid`
      (`EnhancedInputSubsystemInterface.AddMappingContext` _returnvalue "/Game/Inputs/InputMappingContext.InputMappingContext" 0 (struct))
      (bind _outactors (`GameplayStatics.GetAllActorsOfClassWithTag` "/Script/Engine.Actor" "Switch"))
      (for _array_element _outactors
        (set `self.Switcher` _array_element :!label _label))
      (goto _label))))

(event `Initialise UI`
  ;[1 1 1] Creates UI
  (bind _returnvalue (`|CreateWidget` "/Game/UI/BP/WBP_UI.WBP_UI_C"))
  (bind _output_get (set `self.UI` _returnvalue))
  (`UserWidget.AddToViewport` _output_get 0)
  (`/Game/Managers/BPI_UI.UI_Begin` (`self.UI`)))

(event `/Game/Managers/BPI_Controll.CarChangeRequest`
  (params (CarEnum :type "/Game/Vehicles/CarEnums Enum" :default "NewEnumerator0"))
  (`self.CarSwitcher` CarEnum))

(event `EnhancedInput|/Game/Inputs/Switch`
  (params (ActionValue :type Boolean) (ElapsedSeconds :type "Float (double-precision)") (TriggeredSeconds :type "Float (double-precision)") (InputAction :type "InputAction Object Reference" :default "/Game/Inputs/Switch.Switch"))
  ;[1 1 1] Handles Input For the car switching menu
  (:`Started`
    (bind _newstate (message `/Game/Managers/BPI_UI.UI_SwapMenu` (`self.UI`) (`self.SwitchUI`)))
    (set `self.SwitchUI` _newstate)))

(event `EnhancedInput|/Game/Inputs/RightClick`
  (params (ActionValue :type Boolean) (ElapsedSeconds :type "Float (double-precision)") (TriggeredSeconds :type "Float (double-precision)") (InputAction :type "InputAction Object Reference" :default "/Game/Inputs/RightClick.RightClick"))
  (bind (_locationx _locationy) (`self.GetMousePosition`))
  (bind (_x _y) (`KismetMathLibrary.BreakVector2D` (`WidgetLayoutLibrary.GetViewportSize`)))
  (:`Triggered`
    (message `/Game/Managers/BPI_Controll.CameraSwivle` (`self.Car`) (`KismetMathLibrary.MapRangeClamped` _locationx _x 0.0 1.0 -1.0) (`KismetMathLibrary.MapRangeClamped` _locationy _y 0.0 -0.5 0.5)))
  (:`Started`
    (`self.SetMouseLocation` (`KismetMathLibrary.FTrunc` (/ _x 2.0)) (`KismetMathLibrary.FTrunc` (/ _y 2.0)))))

(event `/Game/Managers/BPI_UI.UI_SwitchUIStateChange`
  (params (NewState :type Boolean))
  ;[1 1 1] Handles Input For the car switching menu
  (set `self.SwitchUI` NewState))

(event `EnhancedInput|/Game/Inputs/Ignition`
  (params (ActionValue :type Boolean) (ElapsedSeconds :type "Float (double-precision)") (TriggeredSeconds :type "Float (double-precision)") (InputAction :type "InputAction Object Reference" :default "/Game/Inputs/Ignition.Ignition")))

(event `EnhancedInput|/Game/Inputs/Handbreak`
  (params (ActionValue :type Boolean) (ElapsedSeconds :type "Float (double-precision)") (TriggeredSeconds :type "Float (double-precision)") (InputAction :type "InputAction Object Reference" :default "/Game/Inputs/Handbreak.Handbreak"))
  ;[1 1 1] Inputs done with interfaces
  (:`Triggered`
    (message `/Game/Managers/BPI_Controll.Input_Handbreak` (`self.K2_GetPawn`) ActionValue :!label _label_2))
  (:`Completed`
    (goto _label_2)))

(event `EnhancedInput|/Game/Inputs/Throttle`
  (params (ActionValue :type "Float (double-precision)") (ElapsedSeconds :type "Float (double-precision)") (TriggeredSeconds :type "Float (double-precision)") (InputAction :type "InputAction Object Reference" :default "/Game/Inputs/Throttle.Throttle"))
  ;[1 1 1] Inputs done with interfaces
  (:`Triggered`
    (message `/Game/Managers/BPI_Controll.Input_Forward` (`self.K2_GetPawn`) ActionValue :!label _label_3))
  (:`Completed`
    (goto _label_3)))

(event `EnhancedInput|/Game/Inputs/GearDown`
  (params (ActionValue :type Boolean) (ElapsedSeconds :type "Float (double-precision)") (TriggeredSeconds :type "Float (double-precision)") (InputAction :type "InputAction Object Reference" :default "/Game/Inputs/GearDown.GearDown"))
  ;[1 1 1] Inputs done with interfaces
  (:`Completed`
    (message `/Game/Managers/BPI_Controll.Input_GearDown` (`self.K2_GetPawn`))))

(event `EnhancedInput|/Game/Inputs/GearUp`
  (params (ActionValue :type Boolean) (ElapsedSeconds :type "Float (double-precision)") (TriggeredSeconds :type "Float (double-precision)") (InputAction :type "InputAction Object Reference" :default "/Game/Inputs/GearUp.GearUp"))
  ;[1 1 1] Inputs done with interfaces
  (:`Completed`
    (message `/Game/Managers/BPI_Controll.Input_GearUp` (`self.K2_GetPawn`))))

(event `EnhancedInput|/Game/Inputs/Steering`
  (params (ActionValue :type "Float (double-precision)") (ElapsedSeconds :type "Float (double-precision)") (TriggeredSeconds :type "Float (double-precision)") (InputAction :type "InputAction Object Reference" :default "/Game/Inputs/Steering.Steering"))
  ;[1 1 1] Inputs done with interfaces
  (:`Triggered`
    (message `/Game/Managers/BPI_Controll.Input_Steering` (`self.K2_GetPawn`) ActionValue :!label _label_4))
  (:`Completed`
    (goto _label_4)))

(event `EnhancedInput|/Game/Inputs/Break`
  (params (ActionValue :type "Float (double-precision)") (ElapsedSeconds :type "Float (double-precision)") (TriggeredSeconds :type "Float (double-precision)") (InputAction :type "InputAction Object Reference" :default "/Game/Inputs/Break.Break"))
  ;[1 1 1] Inputs done with interfaces
  (:`Triggered`
    (message `/Game/Managers/BPI_Controll.Input_Breaking` (`self.K2_GetPawn`) ActionValue :!label _label_5))
  (:`Completed`
    (goto _label_5)))

(fn `CarSwitcher`
  (params (CarEnum :type "/Game/Vehicles/CarEnums Enum" :default "NewEnumerator0"))
  (locals (CarClassToSpawn :type "WheeledVehiclePawn Class Reference"))
  (bind (_value _returnvalue) (`BlueprintMapLibrary.Map_Find` (`self.CarMap`) CarEnum))
  (if _returnvalue
    (if (== _value "/Game/Vehicles/VH_Sports/BP_Sports.BP_Sports_C")
      (bind _carmod (message `/Game/Managers/BPI_GetManager.ReturnCarMods` (`GameplayStatics.GetGameInstance`)))
      (switch `/Game/Vehicles/CarMods` _carmod
        (:`NewEnumerator0`
          (set `local.CarClassToSpawn` _value :!label _label))
        (:`NewEnumerator1`
          (set `local.CarClassToSpawn` "/Game/Vehicles/VH_Sports/BP_Sports_SuperCharged.BP_Sports_SuperCharged_C"))
        (:`NewEnumerator2`
          (set `local.CarClassToSpawn` "/Game/Vehicles/VH_Sports/BP_Sports_Turbo.BP_Sports_Turbo_C"))
        (:`NewEnumerator3`
          (set `local.CarClassToSpawn` "/Game/Vehicles/VH_Sports/BP_Sports_Rasied.BP_Sports_Rasied_C")))
      (else
        (goto _label)))
    (else
      (`KismetSystemLibrary.PrintString` "ERROR - Car class not found in MAP - Reverting" true true (struct :`R` 1.0 :`B` 0.039114 :`A` 1.0))
      (bind _output_get (set `local.CarClassToSpawn` "/Game/Vehicles/VH_Sports/BP_Sports.BP_Sports_C"))))
  (bind _returnvalue_2 (`|SpawnActorFromClass` _output_get (`self.GetTransform` (`self.Car`)) "AdjustIfPossibleButAlwaysSpawn" "MultiplyWithRoot" null null))
  (`self.K2_AttachToActor` _returnvalue_2 "None" "SnapToTarget" "KeepWorld" "SnapToTarget")
  (`self.K2_DestroyActor` (`self.Car`))
  (`self.SetUpCar` _returnvalue_2))

(fn `Input_SwitchCar`
  (params (Player :type "PlayerController Object Reference") (CarEnum :type "/Game/Vehicles/CarEnums Enum" :default "NewEnumerator0") (PosToSpawn :type "Transform Structure"))
  (returns (NewCar :type "WheeledVehiclePawn Object Reference"))
  (return null))

(fn `SetUpCar`
  (params (Car :type "WheeledVehiclePawn Object Reference"))
  (bind _mesh (`WheeledVehiclePawn.Mesh` Car))
  (bind _output_get (set `self.Car` Car))
  (`self.Possess` _output_get)
  (bind _materials (message `/Game/Managers/BPI_GetManager.ReturnCarMaterialArray` (`GameplayStatics.GetGameInstance`)))
  (bind _keys (`BlueprintMapLibrary.Map_Keys` _materials))
  (for _array_element _keys
    (switch `/Game/Vehicles/CarMeshElementsEnum` _array_element
      (:`NewEnumerator0`
        (bind _value (`BlueprintMapLibrary.Map_Find` _materials _array_element))
        (`PrimitiveComponent.SetMaterial` _mesh 0 _value))
      (:`NewEnumerator1`
        (`PrimitiveComponent.SetMaterial` _mesh 2 _value))
      (:`NewEnumerator2`
        (`PrimitiveComponent.SetMaterial` _mesh 3 _value))
      (:`NewEnumerator3`
        (`PrimitiveComponent.SetMaterial` _mesh 4 _value)))))

(fn `UI_SwapMenu`
  (params (Active :type Boolean))
  (returns (NewState :type Boolean))
  (return false))

(fn `UserConstructionScript`)