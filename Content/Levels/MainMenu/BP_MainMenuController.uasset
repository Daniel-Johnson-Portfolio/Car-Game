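; Main menu player controller that sets up the menu camera, UI and steering input for the garage car.
; On BeginPlay it spawns and possesses BP_MainMenuCamera, creates WBP_MainMenu with a reference to that camera and shows the cursor.
; If the Enhanced Input subsystem is valid, it adds the mapping context, finds BP_GarageCar in the level and passes it to the widget.
; Steering input is forwarded to the car through InputSteeringMessage.
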(event `self.ReceiveBeginPlay`
  (bind _returnvalue (pcsubsystem `EnhancedInputLocalPlayerSubsystem` self))
  (bind _returnvalue_2 (`|SpawnActorFromClass` "/Game/Levels/MainMenu/BP_MainMenuCamera.BP_MainMenuCamera_C" (`self.Spawn Transform`) "Undefined" "MultiplyWithRoot" null null))
  (`self.Possess` _returnvalue_2)
  (bind _returnvalue_3 (`|CreateWidget` "/Game/UI/BP/WBP_MainMenu.WBP_MainMenu_C"))
  (`UserWidget.AddToViewport` _returnvalue_3 0)
  (set `/Game/UI/BP/WBP_MainMenu.Camera` _returnvalue_2 _returnvalue_3)
  (set `self.bShowMouseCursor` true)
  (`/Engine/EditorBlueprintResources/StandardMacros.IsValid` _returnvalue
    (:`Is Valid`
      (`EnhancedInputSubsystemInterface.AddMappingContext` _returnvalue "/Game/Inputs/InputMappingContext.InputMappingContext" 0 (struct))
      (bind _returnvalue_4 (`GameplayStatics.GetActorOfClass` "/Game/Levels/MainMenu/BP_GarageCar.BP_GarageCar_C"))
      (bind _output_get (set `self.GarageCar` _returnvalue_4))
      (set `/Game/UI/BP/WBP_MainMenu.GarageCar` _output_get _returnvalue_3))))

(event `EnhancedInput|/Game/Inputs/Steering`
  (params (ActionValue :type "Float (double-precision)") (ElapsedSeconds :type "Float (double-precision)") (TriggeredSeconds :type "Float (double-precision)") (InputAction :type "InputAction Object Reference" :default "/Game/Inputs/Steering.Steering"))
  (:`Triggered`
    (message `/Game/Managers/BPI_Controll.Input_Steering` (`self.GarageCar`) ActionValue)))

(fn `UserConstructionScript`)