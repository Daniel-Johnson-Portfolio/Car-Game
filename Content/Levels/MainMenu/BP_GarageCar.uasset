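; Garage preview car for the main menu that rotates with steering input and lets its paint be customised.
; On BeginPlay it puts a dynamic material instance on one mesh slot and caches all BP_Sports actors.
; Colour and emissive events edit that material; red and green are scaled by EmmisiveValue, blue is not.
; ApplyToCar passes the material to every cached sports car and the GameInstance.
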(event `self.ReceiveBeginPlay`
  (bind _returnvalue (`KismetMaterialLibrary.CreateDynamicMaterialInstance` "/Game/Materials/M_PlayerCustomMaterial.M_PlayerCustomMaterial"))
  (bind _output_get (set `self.CustomMaterial` _returnvalue))
  (`PrimitiveComponent.SetMaterial` (`self.SkeletalMesh`) 3 _output_get)
  (bind _returnvalue_2 (`MaterialInstanceDynamic.K2_GetVectorParameterValue` (`self.CustomMaterial`) "RGB"))
  (set `self.ColourVars` _returnvalue_2)
  (bind _outactors (`GameplayStatics.GetAllActorsOfClass` "/Game/Vehicles/VH_Sports/BP_Sports.BP_Sports_C"))
  (set `self.SportsCars` _outactors))

(event `/Game/Managers/BPI_Controll.Input_Steering`
  (params (ActionValue :type "Float (double-precision)"))
  (bind (_returnvalue_roll _returnvalue_pitch _returnvalue_yaw) (`KismetMathLibrary.BreakRotator` (`self.K2_GetActorRotation` self)))
  (`self.K2_SetActorRotation` self (`KismetMathLibrary.MakeRotator` 0.0 0.0 (+ _returnvalue_yaw ActionValue)) false))

(event `Red`
  (params (Value :type "Float (double-precision)"))
  (bind (_r _g _b _a) (`KismetMathLibrary.BreakColor` (`self.ColourVars`)))
  (bind _output_get (set `self.ColourVars` (`KismetMathLibrary.MakeColor` (* Value (`self.EmmisiveValue`)) _g _b _a)))
  (`MaterialInstanceDynamic.SetVectorParameterValue` (`self.CustomMaterial`) "RGB" _output_get))

(event `Green`
  (params (Value :type "Float (double-precision)"))
  (bind (_r _g _b _a) (`KismetMathLibrary.BreakColor` (`self.ColourVars`)))
  (bind _output_get (set `self.ColourVars` (`KismetMathLibrary.MakeColor` _r (* Value (`self.EmmisiveValue`)) _b _a)))
  (`MaterialInstanceDynamic.SetVectorParameterValue` (`self.CustomMaterial`) "RGB" _output_get))

(event `Blue`
  (params (Value :type "Float (double-precision)"))
  (bind (_r _g _b _a) (`KismetMathLibrary.BreakColor` (`self.ColourVars`)))
  (bind _output_get (set `self.ColourVars` (`KismetMathLibrary.MakeColor` _r _g Value _a)))
  (`MaterialInstanceDynamic.SetVectorParameterValue` (`self.CustomMaterial`) "RGB" _output_get))

(event `Emmisive`
  (params (Value :type "Float (double-precision)"))
  (`MaterialInstanceDynamic.SetScalarParameterValue` (`self.CustomMaterial`) "Emmisive" Value))

(event `ApplyToCar`
  (bind _custommaterial (`self.CustomMaterial`))
  (for _array_element (`self.SportsCars`)
    (`/Game/Vehicles/VH_Sports/BP_Sports.Set Custom Material` _array_element _custommaterial)
    (message `/Game/Managers/BPI_GetManager.SetMaterialInstance` (`GameplayStatics.GetGameInstance`) _custommaterial)))

(fn `Input_SwitchCar`
  (params (Player :type "PlayerController Object Reference") (CarEnum :type "/Game/Vehicles/CarEnums Enum" :default "NewEnumerator0") (PosToSpawn :type "Transform Structure"))
  (returns (NewCar :type "WheeledVehiclePawn Object Reference"))
  (return null))

(fn `UserConstructionScript`)