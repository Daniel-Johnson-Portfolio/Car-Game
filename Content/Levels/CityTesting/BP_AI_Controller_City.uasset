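; AI controller that spawns and possesses a BP_Sports car, then self-drives it along a tagged BP_CitySpline in the city level.
; Each Tick it throttles up to MaxSpeed and steers toward a look-ahead spline point by mapping yaw error to input.
; A further look-ahead flags upcoming corners.
; HandlingCheck brakes and caps throttle for corners or oversteer, and narrows steering range for small angles or wheel slip.
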(event `self.ReceiveBeginPlay`
  (`KismetSystemLibrary.PrintString` (`KismetSystemLibrary.GetDisplayName` (`self.Spline`)))
  (bind _returnvalue (`|SpawnActorFromClass` "/Game/Vehicles/VH_Sports/BP_Sports.BP_Sports_C" (`self.SpawnPoint`) "AdjustIfPossibleButAlwaysSpawn" "MultiplyWithRoot" null null))
  (`self.CarSetUp` _returnvalue)
  (bind _materialinstance (message `/Game/Managers/BPI_GetManager.ReturnMaterialInstance` (`GameplayStatics.GetGameInstance`)))
  (`PrimitiveComponent.SetMaterial` (`WheeledVehiclePawn.Mesh` _returnvalue) 3 _materialinstance))

(event `self.ReceiveTick`
  (params (DeltaSeconds :type "Float (single-precision)"))
  (bind _returnvalue (< (`ChaosVehicleMovementComponent.GetForwardSpeedMPH` (`self.Vehicle Movement Component`)) (`self.MaxSpeed`)))
  ;[1 1 1] If Connected car will self drive (Handling Check also needs to be connected)
  (if _returnvalue
    (message `/Game/Managers/BPI_Controll.Input_Forward` (`self.AI_Car`) (`KismetMathLibrary.SelectFloat` 1.0 0.0 _returnvalue)))
  (`self.SettingTarget`)
  (bind (_ai_car _steeringactionvalue) (`self.SteeringCalculation`))
  (message `/Game/Managers/BPI_Controll.Input_Steering` _ai_car _steeringactionvalue)
  ;[1 1 1] Controlls the car when self driving
  (`self.HandlingCheck`))

(event `Break`
  (params (`Break?` :type Boolean))
  (bind _ai_car (`self.AI_Car`))
  ;[1 1 1] Called by handling check applies a half break and a 0.75 throttle limit
  (if `Break?`
    (if (<= (`ChaosVehicleMovementComponent.GetForwardSpeedMPH` (`WheeledVehiclePawn.VehicleMovementComponent` _ai_car)) 10.0)
      (set `/Game/Vehicles/Parent/BP_CarParent.MaxThrottle` 1.0 _ai_car :!label _label)
      (else
        (message `/Game/Managers/BPI_Controll.Input_Breaking` (`self.AI_Car`) 0.5)
        (set `/Game/Vehicles/Parent/BP_CarParent.MaxThrottle` 0.75 _ai_car)))
    (else
      (goto _label))))

(event `LimitSteering`
  (params (`Limit?` :type Boolean))
  ;[1 1 1] Limits steering for small turns
  (if `Limit?`
    (set `self.SteeringA` -0.5)
    (set `self.SteeringB` 0.5)
    (else
      (set `self.SteeringA` -1.0)
      (set `self.SteeringB` 1.0))))

(fn `CarSetUp`
  (params (AI_Car :type "/Game/Vehicles/VH_Sports/BP_Sports Object Reference"))
  (bind _output_get (set `self.AI_Car` AI_Car))
  (set `self.Vehicle Movement Component` (`WheeledVehiclePawn.VehicleMovementComponent` _output_get))
  (set `self.As Chaos Wheeled Vehicle Movement Component` (`/Game/Vehicles/Parent/BP_CarParent.As Chaos Wheeled Vehicle Movement Component` _output_get))
  (`self.Possess` _output_get)
  (set `/Game/Vehicles/Parent/BP_CarParent.ShouldMakeNoise` false _output_get)
  (`ChaosVehicleMovementComponent.SetUseAutomaticGears` (`self.Vehicle Movement Component`) true)
  (`PrimitiveComponent.SetMaterial` (`WheeledVehiclePawn.Mesh` _output_get) 2 "/Game/NotUsed/Systems/Materials/MI_BaseRed.MI_BaseRed"))

(fn `GetNextSplineTarget`
  (params (WorldLocation :type "Vector Structure (by ref)"))
  (returns (ReturnValue :type "Vector Structure"))
  (bind _spline (`self.Spline`))
  (return (`SplineComponent.GetLocationAtDistanceAlongSpline` _spline (+ (`SplineComponent.GetDistanceAlongSplineAtSplineInputKey` _spline (`SplineComponent.FindInputKeyClosestToWorldLocation` _spline WorldLocation)) 500.0) "World")))

(fn `HandlingCheck`
  (bind _as_chaos_wheeled_vehicle_movement_component (`self.As Chaos Wheeled Vehicle Movement Component`))
  (`self.LimitSteering` (`self.AcuteSteeringAngle`))
  (`self.Break` (or (`self.OverSteering?`) (`self.UpCommingCorner`)))
  (for (_ _array_index) (`ChaosWheeledVehicleMovementComponent.Wheels` _as_chaos_wheeled_vehicle_movement_component)
    (bind (_bincontact _contactpoint _physmaterial _normalizedsuspensionlength _springforce _slipangle _bisslipping _slipmagnitude _bisskidding) (`ChaosWheeledVehicleMovementComponent.BreakWheelStatus` (`ChaosWheeledVehicleMovementComponent.GetWheelState` _as_chaos_wheeled_vehicle_movement_component _array_index)))
    (`self.LimitSteering` (or _bisslipping _bisskidding))))

(fn `SettingTarget`
  (set `self.Target` (`SplineComponent.GetLocationAtDistanceAlongSpline` (`self.Spline`) (`self.Distance`) "World")))

(fn `ShouldShiftUp?`
  (params (car :type "/Game/Vehicles/Parent/BP_CarParent Object Reference"))
  (returns (ReturnValue :type Boolean))
  (return (>= (`ChaosWheeledVehicleMovementComponent.GetEngineRotationSpeed` (`self.As Chaos Wheeled Vehicle Movement Component`)) (`/Game/Vehicles/Parent/BP_CarParent.RPM_UpshiftPoint` car))))

(fn `SteeringCalculation`
  (returns (AI_Car :type "/Game/Vehicles/VH_Sports/BP_Sports Object Reference") (SteeringActionValue :type "Float (double-precision)"))
  (bind _car_f (`/Game/Vehicles/VH_Sports/BP_Sports.Car_F` (`self.AI_Car`)))
  (bind _returnvalue (`SceneComponent.K2_GetComponentLocation` _car_f))
  (`self.UpCommingTurn`)
  (bind _returnvalue_2 (`self.GetNextSplineTarget` _returnvalue))
  (bind (_returnvalue_roll _returnvalue_pitch _returnvalue_yaw) (`KismetMathLibrary.BreakRotator` (`KismetMathLibrary.NormalizedDeltaRotator` (`KismetMathLibrary.FindLookAtRotation` _returnvalue _returnvalue_2) (`SceneComponent.K2_GetComponentRotation` _car_f))))
  (set `self.SteeringAngle` _returnvalue_yaw)
  (set `self.AcuteSteeringAngle` (`KismetMathLibrary.InRange_FloatFloat` _returnvalue_yaw -9.0 9.0))
  (bind _returnvalue_3 (`KismetMathLibrary.MapRangeClamped` _returnvalue_yaw -10.0 10.0 (`self.SteeringA`) (`self.SteeringB`)))
  (set `self.OverSteering?` (>= (`KismetMathLibrary.Abs` _returnvalue_3) (`self.MaxSteeringAngle`)))
  (return (`self.AI_Car`) _returnvalue_3))

(fn `UpCommingTurn`
  (bind _spline (`self.Spline`))
  (bind _car_f (`/Game/Vehicles/VH_Sports/BP_Sports.Car_F` (`self.AI_Car`)))
  (bind _returnvalue (`SceneComponent.K2_GetComponentLocation` _car_f))
  (bind (_returnvalue_roll _returnvalue_pitch _returnvalue_yaw) (`KismetMathLibrary.BreakRotator` (`KismetMathLibrary.NormalizedDeltaRotator` (`KismetMathLibrary.FindLookAtRotation` _returnvalue (`SplineComponent.GetLocationAtDistanceAlongSpline` _spline (`SplineComponent.GetDistanceAlongSplineAtSplineInputKey` _spline (+ (`SplineComponent.FindInputKeyClosestToWorldLocation` _spline _returnvalue) 1000.0)) "World")) (`SceneComponent.K2_GetComponentRotation` _car_f))))
  (bind _output_get (set `self.UpcommingSetteringAngle` _returnvalue_yaw))
  (set `self.UpCommingCorner` (== (`KismetMathLibrary.Abs` (`KismetMathLibrary.MapRangeClamped` _output_get -10.0 10.0 (`self.SteeringA`) (`self.SteeringB`))) 0.5)))

(fn `UserConstructionScript`
  (bind _outactors (`GameplayStatics.GetAllActorsOfClassWithTag` "/Game/Levels/CityTesting/BP_CitySpline.BP_CitySpline_C" (`self.SplineTag`)))
  (for _array_element _outactors
    (set `self.RoadSplines` _array_element))
  (bind _roadsplines (`self.RoadSplines`)
    (:`then`
      (set `self.Spline` (`/Game/Levels/CityTesting/BP_CitySpline.Spline` _roadsplines)))
    (:`else`)))