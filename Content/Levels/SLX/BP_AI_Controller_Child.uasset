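; Child of an AI car controller for a level, configuring one specific AI car on Lane1.
; On BeginPlay it sets a fixed spawn transform before running the parent logic, and its construction script assigns the Lane1 spline tag.
; It overrides CarSetUp to pass the Car1 tag to the parent and apply the blue base material to the car mesh.
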(event `self.ReceiveBeginPlay`
  (set `self.SpawnPoint` (`KismetMathLibrary.MakeTransform` (-18200.0 2780.0 250.0) (struct :`Yaw` -95.0)))
  (`parent.ReceiveBeginPlay`))

(fn `CarSetUp`
  (params (AI_Car :type "/Game/Vehicles/VH_Sports/BP_Sports Object Reference") (Tag :type Name))
  (`parent.CarSetUp` AI_Car "Car1")
  (`PrimitiveComponent.SetMaterial` (`WheeledVehiclePawn.Mesh` AI_Car) 2 "/Game/NotUsed/Systems/Materials/MI_BaseBlue.MI_BaseBlue"))

(fn `UserConstructionScript`
  (set `self.SplineTag` "Lane1")
  (`parent.UserConstructionScript`))