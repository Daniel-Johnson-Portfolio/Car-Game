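; Player controller for the SLX level that drives two cars from one local controller, one throttle input per player.
; On BeginPlay it finds the cars by tag, creates the SLX widget, possesses the shared camera pawn and adds the input mapping context.
; Each throttle action sends forward input to its car, releasing the brake while held and applying full brake when let go.
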(event `self.ReceiveBeginPlay`
  (bind _returnvalue (pcsubsystem `EnhancedInputLocalPlayerSubsystem` self))
  (`self.CarSetUp` "Car1")
  (`self.CarSetUp` "Car2")
  (`self.Initialise UI`)
  (bind _returnvalue_2 (`GameplayStatics.GetActorOfClass` "/Game/Levels/SLX/BP_CameraPawn.BP_CameraPawn_C"))
  (`self.Possess` _returnvalue_2)
  (`/Engine/EditorBlueprintResources/StandardMacros.IsValid` _returnvalue
    (:`Is Valid`
      (`EnhancedInputSubsystemInterface.AddMappingContext` _returnvalue "/Game/Inputs/InputMappingContext.InputMappingContext" 1 (struct)))))

(event `Initialise UI`
  ;[1 1 1] Creates UI
  (bind _returnvalue (`|CreateWidget` "/Game/UI/BP/WBP_SLX.WBP_SLX_C"))
  (bind _output_get (set `self.UI` _returnvalue))
  (`UserWidget.AddToViewport` _output_get 0))

(event `EnhancedInput|/Game/Inputs/Throttle`
  (params (ActionValue :type "Float (double-precision)") (ElapsedSeconds :type "Float (double-precision)") (TriggeredSeconds :type "Float (double-precision)") (InputAction :type "InputAction Object Reference" :default "/Game/Inputs/Throttle.Throttle"))
  (bind _car1 (`self.Car1`))
  (:`Triggered`
    (set `self.Plr1Accel?` true)
    (message `/Game/Managers/BPI_Controll.Input_Forward` _car1 ActionValue :!label _label)
    (if (`self.Plr1Accel?`)
      (message `/Game/Managers/BPI_Controll.Input_Breaking` _car1 0.0)
      (else
        (message `/Game/Managers/BPI_Controll.Input_Breaking` _car1 1.0))))
  (:`Completed`
    (set `self.Plr1Accel?` false)
    (goto _label)))

(event `EnhancedInput|/Game/Inputs/Plr2_Throttle`
  (params (ActionValue :type "Float (double-precision)") (ElapsedSeconds :type "Float (double-precision)") (TriggeredSeconds :type "Float (double-precision)") (InputAction :type "InputAction Object Reference" :default "/Game/Inputs/Plr2_Throttle.Plr2_Throttle"))
  (bind _car2 (`self.Car2`))
  (:`Triggered`
    (set `self.Plr2Accel?` true)
    (message `/Game/Managers/BPI_Controll.Input_Forward` _car2 ActionValue :!label _label_2)
    (if (`self.Plr2Accel?`)
      (message `/Game/Managers/BPI_Controll.Input_Breaking` _car2 0.0)
      (else
        (message `/Game/Managers/BPI_Controll.Input_Breaking` _car2 1.0))))
  (:`Completed`
    (set `self.Plr2Accel?` false)
    (goto _label_2)))

(fn `CarSetUp`
  (params (Tag :type Name))
  (bind _outactors (`GameplayStatics.GetAllActorsOfClassWithTag` "/Game/Vehicles/Parent/BP_CarParent.BP_CarParent_C" Tag))
  (for _array_element _outactors
    (if (== Tag "Car1")
      (set `self.Car1` _array_element)
      (else
        (set `self.Car2` _array_element))))
  (return))

(fn `UserConstructionScript`)