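; BP_Goal is a goal trigger that signals a win when a car reaches it.
; On Cube overlap, it checks whether the other actor's class derives from BP_CarParent, then calls UIWinConditionMessage on its GoalUI reference.
; Debug strings print on both branches, and the UISwapMenu function from UI_SwapMenu is a stub returning false.
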(event `self.ReceiveBeginPlay`)

(event `self.Cube.OnComponentBeginOverlap`
  (params (OverlappedComponent :type "PrimitiveComponent Object Reference") (OtherActor :type "Actor Object Reference") (OtherComp :type "PrimitiveComponent Object Reference") (OtherBodyIndex :type Integer) (bFromSweep :type Boolean) (SweepResult :type "HitResult Structure (by ref)"))
  (bind _goalui (`self.GoalUI`))
  (if (`KismetMathLibrary.ClassIsChildOf` (`GameplayStatics.GetObjectClass` OtherActor) "/Game/Vehicles/Parent/BP_CarParent.BP_CarParent_C")
    (`KismetSystemLibrary.PrintString` (`KismetSystemLibrary.GetDisplayName` _goalui))
    (message `/Game/BPI_UI.UI_WinCondition` _goalui)
    (else
      (`KismetSystemLibrary.PrintString` "False"))))

(fn `UI_SwapMenu`
  (params (Active :type Boolean))
  (returns (NewState :type Boolean))
  (return false))

(fn `UserConstructionScript`)