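; Camera pawn that keeps two cars in a shared view by following their midpoint at a fixed rotation.
; On BeginPlay it attaches to the first BP_CarParent found and caches all such cars, though Tick uses only the first two.
; Each tick it raises or lowers its clamped height offset depending on MaxDistance, stepping by car separation without delta-time scaling, and prints the offset for debugging.
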(event `self.ReceiveBeginPlay`
  (bind _returnvalue (`GameplayStatics.GetActorOfClass` "/Game/Vehicles/Parent/BP_CarParent.BP_CarParent_C"))
  (`self.K2_AttachToActor` _returnvalue "None" "KeepRelative" "KeepRelative" "KeepRelative")
  (bind _outactors (`GameplayStatics.GetAllActorsOfClass` "/Game/Vehicles/Parent/BP_CarParent.BP_CarParent_C"))
  (for _index (range (+ (`KismetArrayLibrary.Array_Length` _outactors) 1))
    (`KismetArrayLibrary.Array_Add` (`self.Cars`) (`|GetArrayItem` _outactors _index))))

(event `self.ReceiveTick`
  (params (DeltaSeconds :type "Float (single-precision)"))
  (bind _cars (`self.Cars`))
  (bind _returnvalue (`self.K2_GetActorLocation` (`|GetArrayItem` _cars 1)))
  (bind _returnvalue_2 (`self.K2_GetActorLocation` (`|GetArrayItem` _cars)))
  (bind _returnvalue_3 (`KismetMathLibrary.Vector_Distance` _returnvalue_2 _returnvalue))
  (bind (_returnvalue_x _returnvalue_y) (`KismetMathLibrary.BreakVector` (/ (+ _returnvalue_2 _returnvalue) 2)))
  (`self.K2_SetActorLocationAndRotation` self (`KismetMathLibrary.MakeVector` _returnvalue_x _returnvalue_y (+ (`self.DefaultHeight`) (`self.HeightOffset`))) (struct :`Yaw` 270.0) false false)
  (set `self.OffsetChange` (/ _returnvalue_3 1500.0))
  (`KismetSystemLibrary.PrintString` (`KismetStringLibrary.Conv_DoubleToString` (`self.HeightOffset`)))
  (if (>= _returnvalue_3 (`self.MaxDistance`))
    (set `self.HeightOffset` (`KismetMathLibrary.FClamp` (+ (`self.HeightOffset`) (`self.OffsetChange`)) 0.0 15000.0))
    (else
      (set `self.HeightOffset` (`KismetMathLibrary.FClamp` (- (`self.HeightOffset`) (`self.OffsetChange`)) 0.0 15000.0)))))

(fn `UserConstructionScript`)