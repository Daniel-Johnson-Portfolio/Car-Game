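; BP_AiGMController is a controller that creates the game UI and forwards player driving input to a car.
; On BeginPlay it finds a BP_CarParent, creates WBP_UI, possesses BP_CameraPawn and immediately the car, then adds an Enhanced Input mapping context.
; Throttle, steering and brake actions pass their values to the stored car through message calls on both Triggered and Completed.
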(event `self.ReceiveBeginPlay`
  (bind _returnvalue (pcsubsystem `EnhancedInputLocalPlayerSubsystem` self))
  (bind _returnvalue_2 (`GameplayStatics.GetActorOfClass` "/Game/Vehicles/Parent/BP_CarParent.BP_CarParent_C"))
  (bind _output_get (set `self.CurrentAIcar` _returnvalue_2))
  (`self.Initialise UI`)
  (bind _returnvalue_3 (`GameplayStatics.GetActorOfClass` "/Game/BP_CameraPawn.BP_CameraPawn_C"))
  (`self.Possess` _returnvalue_3)
  (`self.Possess` _output_get)
  (`/Engine/EditorBlueprintResources/StandardMacros.IsValid` _returnvalue
    (:`Is Valid`
      (`EnhancedInputSubsystemInterface.AddMappingContext` _returnvalue "/Game/Inputs/InputMappingContext.InputMappingContext" 1 (struct)))))

(event `Initialise UI`
  ;[1 1 1] Creates UI
  (bind _returnvalue (`|CreateWidget` "/Game/WBP_UI.WBP_UI_C"))
  (bind _output_get (set `self.UI` _returnvalue))
  (`UserWidget.AddToViewport` _output_get 0)
  (`/Game/BPI_UI.UI_Begin` _returnvalue))

(event `EnhancedInput|/Game/Inputs/Throttle`
  (params (ActionValue :type "Float (double-precision)") (ElapsedSeconds :type "Float (double-precision)") (TriggeredSeconds :type "Float (double-precision)") (InputAction :type "InputAction Object Reference" :default "/Game/Inputs/Throttle.Throttle"))
  (:`Triggered`
    (message `/Game/BPI_Controll.Input_Forward` (`self.CurrentAIcar`) ActionValue :!label _label))
  (:`Completed`
    (goto _label)))

(event `EnhancedInput|/Game/Inputs/Steering`
  (params (ActionValue :type "Float (double-precision)") (ElapsedSeconds :type "Float (double-precision)") (TriggeredSeconds :type "Float (double-precision)") (InputAction :type "InputAction Object Reference" :default "/Game/Inputs/Steering.Steering"))
  (:`Triggered`
    (message `/Game/BPI_Controll.Input_Steering` (`self.CurrentAIcar`) ActionValue :!label _label_2))
  (:`Completed`
    (goto _label_2)))

(event `EnhancedInput|/Game/Inputs/Break`
  (params (ActionValue :type "Float (double-precision)") (ElapsedSeconds :type "Float (double-precision)") (TriggeredSeconds :type "Float (double-precision)") (InputAction :type "InputAction Object Reference" :default "/Game/Inputs/Break.Break"))
  (:`Triggered`
    (message `/Game/BPI_Controll.Input_Breaking` (`self.CurrentAIcar`) ActionValue :!label _label_3))
  (:`Completed`
    (goto _label_3)))

(fn `UserConstructionScript`)