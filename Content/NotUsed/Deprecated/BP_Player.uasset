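; Deprecated player Blueprint that acts as an input relay for driving a car through interface messages.
; On BeginPlay it creates the UI, adds the input mapping and attaches itself to each BPI_Controll actor found, keeping the last as Car.
; Enhanced Input events forward throttle, brake, steering, handbrake and gear shifts to that Car.
; "Switch"-tagged actors are cached, but the car-switching call is disconnected, and debug prints remain.
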(event `self.ReceiveBeginPlay`
  (bind _returnvalue (pcsubsystem `EnhancedInputLocalPlayerSubsystem` (`GameplayStatics.GetPlayerController` 0)))
  (bind _returnvalue_2 (`|CreateWidget` "/Game/UI/BP/WBP_UI.WBP_UI_C"))
  (`UserWidget.AddToViewport` _returnvalue_2 0)
  (`/Engine/EditorBlueprintResources/StandardMacros.IsValid` _returnvalue
    (:`Is Valid`
      (`EnhancedInputSubsystemInterface.AddMappingContext` _returnvalue "/Game/Inputs/InputMappingContext.InputMappingContext" 0 (struct))
      (bind _outactors (`GameplayStatics.GetAllActorsWithInterface` "/Game/Managers/BPI_Controll.BPI_Controll_C"))
      (for _array_element _outactors
        (bind _output_get (set `self.Car` _array_element :!label _label))
        (`self.K2_AttachToActor` _output_get "None" "SnapToTarget" "KeepWorld" "SnapToTarget")
        (bind _outactors_2 (`GameplayStatics.GetAllActorsOfClassWithTag` "/Script/Engine.Actor" "Switch"))
        (for _array_element_2 _outactors_2
          (set `self.Switcher` _array_element_2 :!label _label_2)
          (`KismetSystemLibrary.PrintString` "Hello"))
        (goto _label_2))
      (goto _label))))

(event `EnhancedInput|/Game/Inputs/Switch`
  (params (ActionValue :type Boolean) (ElapsedSeconds :type "Float (double-precision)") (TriggeredSeconds :type "Float (double-precision)") (InputAction :type "InputAction Object Reference" :default "/Game/Inputs/Switch.Switch")))

(event `EnhancedInput|/Game/Inputs/Ignition`
  (params (ActionValue :type Boolean) (ElapsedSeconds :type "Float (double-precision)") (TriggeredSeconds :type "Float (double-precision)") (InputAction :type "InputAction Object Reference" :default "/Game/Inputs/Ignition.Ignition")))

(event `EnhancedInput|/Game/Inputs/Handbreak`
  (params (ActionValue :type Boolean) (ElapsedSeconds :type "Float (double-precision)") (TriggeredSeconds :type "Float (double-precision)") (InputAction :type "InputAction Object Reference" :default "/Game/Inputs/Handbreak.Handbreak"))
  (:`Triggered`
    (message `/Game/Managers/BPI_Controll.Input_Handbreak` (`self.Car`) ActionValue :!label _label_3))
  (:`Completed`
    (goto _label_3)))

(event `EnhancedInput|/Game/Inputs/Throttle`
  (params (ActionValue :type "Float (double-precision)") (ElapsedSeconds :type "Float (double-precision)") (TriggeredSeconds :type "Float (double-precision)") (InputAction :type "InputAction Object Reference" :default "/Game/Inputs/Throttle.Throttle"))
  (:`Triggered`
    (message `/Game/Managers/BPI_Controll.Input_Forward` (`self.Car`) ActionValue :!label _label_4))
  (:`Completed`
    (goto _label_4)))

(event `EnhancedInput|/Game/Inputs/GearDown`
  (params (ActionValue :type Boolean) (ElapsedSeconds :type "Float (double-precision)") (TriggeredSeconds :type "Float (double-precision)") (InputAction :type "InputAction Object Reference" :default "/Game/Inputs/GearDown.GearDown"))
  (:`Completed`
    (message `/Game/Managers/BPI_Controll.Input_GearDown` (`self.Car`))))

(event `EnhancedInput|/Game/Inputs/GearUp`
  (params (ActionValue :type Boolean) (ElapsedSeconds :type "Float (double-precision)") (TriggeredSeconds :type "Float (double-precision)") (InputAction :type "InputAction Object Reference" :default "/Game/Inputs/GearUp.GearUp"))
  (:`Completed`
    (message `/Game/Managers/BPI_Controll.Input_GearUp` (`self.Car`))))

(event `EnhancedInput|/Game/Inputs/Steering`
  (params (ActionValue :type "Float (double-precision)") (ElapsedSeconds :type "Float (double-precision)") (TriggeredSeconds :type "Float (double-precision)") (InputAction :type "InputAction Object Reference" :default "/Game/Inputs/Steering.Steering"))
  (:`Triggered`
    (message `/Game/Managers/BPI_Controll.Input_Steering` (`self.Car`) ActionValue :!label _label_5))
  (:`Completed`
    (goto _label_5)))

(event `EnhancedInput|/Game/Inputs/Break`
  (params (ActionValue :type "Float (double-precision)") (ElapsedSeconds :type "Float (double-precision)") (TriggeredSeconds :type "Float (double-precision)") (InputAction :type "InputAction Object Reference" :default "/Game/Inputs/Break.Break"))
  (:`Triggered`
    (message `/Game/Managers/BPI_Controll.Input_Breaking` (`self.Car`) ActionValue :!label _label_6))
  (:`Completed`
    (goto _label_6)))

(event `self.ReceiveTick`
  (params (DeltaSeconds :type "Float (single-precision)"))
  (`KismetSystemLibrary.PrintString` (`KismetSystemLibrary.GetDisplayName` (`self.Car`))))

(fn `UserConstructionScript`)