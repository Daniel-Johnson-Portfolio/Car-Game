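; BP_BasePlatform is a base moving platform that can be switched on and off through interaction.
; It caches its start location on BeginPlay and activates immediately if IsEnabled is set.
; A timeline lerps it toward TargetLoc, treated as an offset from the start, moving it without sweep.
; Interact toggles between Activate and Disable, which stops the timeline in place so Play resumes from there.
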(event `self.ReceiveBeginPlay`
  (set `self.StartLoc` (`self.K2_GetActorLocation`))
  (if (`self.IsEnabled`)
    (`self.Activate`)))

(event `Activate`
  (bind _startloc (`self.StartLoc`))
  (set `self.IsEnabled` true)
  (bind (_direction _movealpha) (`Timeline|MovementTimeline` :!label _label)
    (:`Update`
      (`self.K2_SetActorLocation` (`KismetMathLibrary.VLerp` _startloc (+ _startloc (`self.TargetLoc`)) _movealpha)))))

(event `Disable`
  (set `self.IsEnabled` false)
  (goto _label :!via `Stop`))

(event `Interact`
  (if (`self.IsEnabled`)
    (`self.Disable`)
    (else
      (`self.Activate`))))

(fn `UserConstructionScript`)