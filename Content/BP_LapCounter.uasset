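; BP_LapCounter is a lap trigger that counts laps for two tagged cars in a race.
; On BeginPlay it finds the WBP_SLX widget and stores it as SLXUI.
; When an actor overlaps its Box, it matches the actor's Car1 or Car2 tag and increments that car's lap count on the Gamemode.
; It then sends the lap message to the widget and has the Gamemode check the lap counters.
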(event `self.ReceiveBeginPlay`
  (bind _foundwidgets (`WidgetBlueprintLibrary.GetAllWidgetsOfClass` "/Game/WBP_SLX.WBP_SLX_C"))
  (for _array_element _foundwidgets
    (set `self.SLX_UI` _array_element)))

(event `self.Box.OnComponentHit`
  (params (HitComponent :type "PrimitiveComponent Object Reference") (OtherActor :type "Actor Object Reference") (OtherComp :type "PrimitiveComponent Object Reference") (NormalImpulse :type "Vector Structure") (Hit :type "HitResult Structure (by ref)")))

(event `self.Box.OnComponentBeginOverlap`
  (params (OverlappedComponent :type "PrimitiveComponent Object Reference") (OtherActor :type "Actor Object Reference") (OtherComp :type "PrimitiveComponent Object Reference") (OtherBodyIndex :type Integer) (bFromSweep :type Boolean) (SweepResult :type "HitResult Structure (by ref)"))
  (bind _slx_ui (`self.SLX_UI`))
  (for _array_element (`Actor.Tags` OtherActor)
    (if (== _array_element "Car1")
      (bind _result (`/Engine/EditorBlueprintResources/StandardMacros.IncrementInt` (`/Game/GM_AiCar.CurrentLapCar1` (`self.Gamemode`)))
        (:`  `
          (set `/Game/GM_AiCar.CurrentLapCar1` _result (`self.Gamemode`))
          (message `/Game/BPI_UI.UI_Lap` _slx_ui _result _array_element)
          (`/Game/GM_AiCar.CheckLapCounters` (`self.Gamemode`) _slx_ui :!label _label)))
      (elif (== _array_element "Car2")
        (bind _result_2 (`/Engine/EditorBlueprintResources/StandardMacros.IncrementInt` (`/Game/GM_AiCar.CurrentLapCar2` (`self.Gamemode`)))
          (:`  `
            (set `/Game/GM_AiCar.CurrentLapCar2` _result_2 (`self.Gamemode`))
            (message `/Game/BPI_UI.UI_Lap` (`self.SLX_UI`) _result_2 _array_element)
            (goto _label)))))))

(fn `UserConstructionScript`)